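; B_WeaponDecalBase is a weapon effect actor that spawns bullet impact decals matched to the surface type hit.
; FireEffect looks up the material in DT_BulletDecalData by surface enum name, then spawns a short-lived decal along the impact normal with random size and roll.
; A retriggerable delay loop, restarted by each call, polls the last spawned decal and destroys the actor once that decal is no longer valid.
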(event EventBeginPlay)

(event Collision|EventActorBeginOverlap
  (params (OtherActor :type Actor%20Object%20Reference)))

(event EventTick
  (params (DeltaSeconds :type Float%20%28single-precision%29)))

(event EventFireEffect
  (params (IsFP :type Boolean) (Location :type Vector :default "0, 0, 0") (ImpactNormal :type Vector :default "0, 0, 0") (SurfaceType :type EPhysicalSurface%20Enum :default "SurfaceType_Default"))
  (Utilities|FlowControl|Sequence
    (:then_0
      (bind _returnvalue (Utilities|GetDataTableRow "/Game/RTFPS/PhysicsData/DT_BulletDecalData.DT_BulletDecalData" (Utilities|String|StringToName (Utilities|String|EnumtoString SurfaceType)))
        (:then
          (bind _returnvalue_2 (Rendering|Decal|SpawnDecalatLocation (Utilities|Struct|BreakS_BulletDecalInfo _returnvalue) (Math|Conversions|ToVector(Float) (Math|Random|RandomFloatinRange 1.0 1.5)) Location (Math|Conversions|RotationFromXVector ImpactNormal) 1e+01))
          (Transformation|AddLocalRotation _returnvalue_2 (Math|Rotator|MakeRotator (Math|Random|RandomFloatinRange 0.0 3.6e+02) 0.0 0.0) false false)
          (Variables|Default|SetLastSpawnedDecal _returnvalue_2))))
    (:then_1
      ;[1 1 1] ResetEffectPool
      (Utilities|FlowControl|RetriggerableDelay 2.0 :!label _label)
      (if (Utilities|IsValid (Variables|Default|GetLastSpawnedDecal))
        (goto _label)
        (else
          (Actor|DestroyActor))))))

(fn ConstructionScript)