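; Base weapon actor for an FPS, serving as either the first-person or third-person copy of a weapon according to IsFPWeapon.
; One tick after BeginPlay, it applies that flag to WeaponMesh and all child primitive components.
; First-person copies are owner-only and shadowless, while third-person copies are hidden from the owner but still cast shadows through hidden shadow.
; Fire only plays FireMontage on the weapon mesh at PlayRate.
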(event Custom|Fire
  (Animation|Montage|PlayMontage (Variables|Default|GetWeaponMesh) (Variables|Default|GetFireMontage) (Variables|Default|GetPlay%20Rate)))

(event EventBeginPlay
  (bind _weaponmesh (Variables|Default|GetWeaponMesh))
  (bind _weaponmesh_2 (Variables|Default|GetWeaponMesh))
  (bind _weaponmesh_3 (Variables|Default|GetWeaponMesh))
  (Utilities|FlowControl|DelayUntilNextTick)
  (Utilities|FlowControl|Sequence
    (:then_0
      ;[1 1 1] Hide FP Mesh Shadow
      (Rendering|SetCastShadow _weaponmesh_2 (not (Variables|Default|GetIsFPWeapon)))
      (for _array_element (Components|GetChildrenComponents _weaponmesh_2 true)
        (bind _asprimitive_component (Utilities|Casting|CastToPrimitiveComponent _array_element))
        (Rendering|SetCastShadow _asprimitive_component (not (Variables|Default|GetIsFPWeapon)))))
    (:then_1
      ;[1 1 1] Show FP Mesh to Only Owner/Hide FP Mesh to Owner
      (Class|PrimitiveComponent|SetOwnerNoSee _weaponmesh (not (Variables|Default|GetIsFPWeapon)))
      (Rendering|SetOnlyOwnerSee _weaponmesh (Variables|Default|GetIsFPWeapon) :!class /Script/Engine.PrimitiveComponent)
      (for _array_element_2 (Components|GetChildrenComponents _weaponmesh true)
        (bind _asprimitive_component_2 (Utilities|Casting|CastToPrimitiveComponent _array_element_2))
        (Class|PrimitiveComponent|SetOwnerNoSee _asprimitive_component_2 (not (Variables|Default|GetIsFPWeapon)))
        (Rendering|SetOnlyOwnerSee _asprimitive_component_2 (Variables|Default|GetIsFPWeapon) :!class /Script/Engine.PrimitiveComponent)))
    (:then_2
      ;[1 1 1] Show TP Mesh Shadow
      (Class|PrimitiveComponent|SetCastHiddenShadow _weaponmesh_3 (not (Variables|Default|GetIsFPWeapon)))
      (for _array_element_3 (Components|GetChildrenComponents _weaponmesh_3 true)
        (bind _asprimitive_component_3 (Utilities|Casting|CastToPrimitiveComponent _array_element_3))
        (Class|PrimitiveComponent|SetCastHiddenShadow _asprimitive_component_3 (not (Variables|Default|GetIsFPWeapon)))))))

(event Collision|EventActorBeginOverlap
  (params (OtherActor :type Actor%20Object%20Reference)))

(event EventTick
  (params (DeltaSeconds :type Float%20%28single-precision%29)))

(fn ConstructionScript)