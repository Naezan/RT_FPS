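; Base weapon-fire effect actor that plays Niagara muzzle flash and shell eject effects on a weapon's skeletal mesh.
; FireEffect spawns FX only for first-person on the autonomous proxy or third-person on simulated proxies, judged by the owning pawn's role.
; Each shot spawns a flash, while an active shell system is reused by toggling its User.Trigger bool.
; A retriggerable delay destroys the actor once the last effects are gone.
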(event EventBeginPlay)

(event EventFireEffect
  (params (IsFP :type Boolean))
  (Variables|Default|SetIs%20FP IsFP)
  (Utilities|FlowControl|Sequence
    (:then_0
      (if (CallFunction|CanSpawnFX)
        (Utilities|FlowControl|Sequence
          (:then_0
            ;[1 1 1] Register Muzzle Flash Effect
            (bind _returnvalue (Niagara|SpawnSystemAttached (Variables|Niagara-MuzzleFlash|GetMuzzleFlash) (Variables|Default|GetSkeletalMeshComponent) "None" (.Location (Math|Transform|BreakTransform (Transformation|GetSocketTransform (Variables|Default|GetSkeletalMeshComponent) "Muzzle" "RTS_Actor"))) "0.000000,90.000000,0.000000" "KeepRelativeOffset" true))
            (Variables|Niagara-MuzzleFlash|SetLastAttachedMuzzleFlash _returnvalue))
          (:then_1
            ;[1 1 1] Register Shell Eject Effect
            (Utilities|IsValid (Variables|Niagara-ShellEject|GetLastAttachedShellEject)
              (:Is%20Valid
                (if (Components|Activation|IsActive (Variables|Niagara-ShellEject|GetLastAttachedShellEject))
                  _
                  (else
                    (bind _returnvalue_2 (Niagara|SpawnSystemAttached (Variables|Niagara-ShellEject|GetShellEject) (Variables|Default|GetSkeletalMeshComponent) "None" (.Location (Math|Transform|BreakTransform (Transformation|GetSocketTransform (Variables|Default|GetSkeletalMeshComponent) "ShellEject" "RTS_Actor"))) "0.000000,90.000000,0.000000" "KeepRelativeOffset" true :!label _label))
                    (Variables|Niagara-ShellEject|SetLastAttachedShellEject _returnvalue_2)
                    (Class|NiagaraComponent|SetVariableStaticMesh (Variables|Niagara-ShellEject|GetLastAttachedShellEject) "User.ShellEjectStaticMesh" (Variables|Niagara-ShellEject|GetShellEjectMesh))
                    (Variables|Niagara-ShellEject|SetFlipFlopTrigger false))))
              (:Is%20Not%20Valid
                (goto _label)))
            (Variables|Niagara-ShellEject|SetFlipFlopTrigger (not (Variables|Niagara-ShellEject|GetFlipFlopTrigger)))
            (Class|NiagaraComponent|SetVariableBool (Variables|Niagara-ShellEject|GetLastAttachedShellEject) "User.Trigger" (Variables|Niagara-ShellEject|GetFlipFlopTrigger))))))
    (:then_1
      ;[1 1 1] ResetEffectPool
      (Utilities|FlowControl|RetriggerableDelay 2.0 :!label _label_2)
      (if (or (Utilities|IsValid (Variables|Niagara-MuzzleFlash|GetLastAttachedMuzzleFlash)) (Utilities|IsValid (Variables|Niagara-ShellEject|GetLastAttachedShellEject)))
        (goto _label_2)
        (else
          (Actor|DestroyActor))))))

(fn ConstructionScript)

(fn GetOwnerWeapon
  (return (Components|GetOwner (Variables|Default|GetSkeletalMeshComponent))))

(fn GetOwnedPlayer
  (bind _skeletalmeshcomponent (Variables|Default|GetSkeletalMeshComponent))
  (bind _returnvalue (Components|GetOwner _skeletalmeshcomponent))
  (Utilities|IsValid _returnvalue
    (:Is%20Valid
      (bind _aspawn (Utilities|Casting|CastToPawn (Components|GetOwner _returnvalue))
        (:then
          (return _aspawn))
        (:CastFailed
          _)))
    (:Is%20Not%20Valid
      _))
  (return 0))

(fn IsControlledPlayer
  (if (Utilities|Enum|Equal(Enum) (Networking|GetLocalRole (CallFunction|GetOwnedPlayer)) "ROLE_AutonomousProxy")
    (return true)
    (else
      (return false))))

(fn IsSimulatedProxy
  (if (Utilities|Enum|Equal(Enum) (Networking|GetLocalRole (CallFunction|GetOwnedPlayer)) "ROLE_SimulatedProxy")
    (return true)
    (else
      (return false))))

(fn CanSpawnFX
  (if (Variables|Default|GetIs%20FP)
    (if (CallFunction|IsControlledPlayer) ; Spawn Only LocalWeapon
      _
      (else
        (return false)))
    (elif (CallFunction|IsSimulatedProxy) ; Spawn Only SimulatedProxyWeapon
      _
      (else
        (return false))))
  (return true))