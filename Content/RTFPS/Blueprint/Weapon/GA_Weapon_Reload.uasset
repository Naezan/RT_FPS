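; Gameplay ability that reloads a weapon, allowed only when the equipment component's current magazine capacity exceeds one.
; Activation adds a loose BlockFire tag, removed on end, and plays the reload montage as both normal and first-person montage.
; The authority waits for a ReloadComplete gameplay event, then loads the next magazine through RFEquipmentComponent and ends the ability.
; Montage completion ends it locally, while interruption, cancellation or a missing montage ends it fully.
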(event Ability|EventActivateAbility
  ;[1 1 1] Block fire when reloading
  (Ability|GameplayEffect|AddLooseGameplayTags (Ability|GetOwningActorfromActorInfo) (GameplayTags|MakeLiteralGameplayTagContainer "(GameplayTags=((TagName=\"Ability.Weapon.Event.BlockFire\")))"))
  (bind _reloadmontage (Variables|Default|GetReloadMontage)
    (:then
      (|RFPlayMontageandWaitProxy "None" _reloadmontage _reloadmontage 1.0 "None" true 1.0 0.0 false
        (:then
          (Ability|HasAuthority
            (:True
              (Ability|Tasks|WaitGameplayEvent "(TagName=\"Ability.Weapon.Event.ReloadComplete\")" 0 true
                (:EventReceived
                  (CallFunction|ReloadMagazine)
                  (Ability|EndAbility))))))
        (:OnCompleted
          (Ability|EndAbilityLocally))
        (:OnInterrupted
          ;[1 1 1] End ability when dead
          (Ability|EndAbility :!label _label))
        (:OnCancelled
          (goto _label))))
    (:else
      (goto _label))))

(event Ability|EventOnEndAbility
  (params (bWasCancelled :type Boolean))
  (Ability|GameplayEffect|RemoveLooseGameplayTags (Ability|GetOwningActorfromActorInfo) (GameplayTags|MakeLiteralGameplayTagContainer "(GameplayTags=((TagName=\"Ability.Weapon.Event.BlockFire\")))")))

(fn ReloadMagazine
  (bind _returnvalue (Ability|GetAvatarActorfromActorInfo))
  (bind _returnvalue_2 (Actor|GetComponentbyClass _returnvalue "/Script/RT_FPS.RFEquipmentComponent"))
  (Utilities|IsValid _returnvalue
    (:Is%20Valid
      (Utilities|IsValid _returnvalue_2
        (:Is%20Valid
          (Class|RFEquipmentComponent|ReloadNextMagazine _returnvalue_2))))))

(fn K2CanActivateAbility
  (params (ActorInfo :type Gameplay%20Ability%20Actor%20Info%20Structure) (Handle :type Gameplay%20Ability%20Spec%20Handle%20Structure))
  (bind _avataractor (Utilities|Struct|BreakGameplayAbilityActorInfo ActorInfo))
  (bind _returnvalue (Actor|GetComponentbyClass _avataractor "/Script/RT_FPS.RFEquipmentComponent"))
  (Utilities|IsValid _avataractor
    (:Is%20Valid
      (Utilities|IsValid _returnvalue
        (:Is%20Valid
          (return "" (> (Class|RFEquipmentComponent|GetCurrentMagazineCapacity _returnvalue) 1)))
        (:Is%20Not%20Valid
          _)))
    (:Is%20Not%20Valid
      _))
  (return "" false))