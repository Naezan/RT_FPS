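; Gameplay ability that switches a weapon's fire select mode up or down, as set by IsUpSelect.
; While active it adds a non-replicated BlockFire loose tag to the owning actor and removes it when the ability ends.
; It plays FireSelectMontage, changing the mode on both first-person and third-person weapon actors as playback starts.
; The ability ends when the montage finishes or is interrupted, or immediately without a mode change if no montage is valid.
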(event Ability|EventActivateAbility
  ;[1 1 1] Block fire when reloading
  (|CallParentFunction)
  (Ability|GameplayEffect|AddLooseGameplayTags (Ability|GetOwningActorfromActorInfo) (GameplayTags|MakeLiteralGameplayTagContainer "(GameplayTags=((TagName=\"Ability.Weapon.Event.BlockFire\")))"))
  (bind _fireselectmontage (Variables|Default|GetFireSelectMontage)
    (:then
      (|RFPlayMontageandWaitProxy "None" _fireselectmontage 0 1.0 "None" true 1.0 0.0 false
        (:then
          (CallFunction|ChangeSelectMode (Class|RFGameplayAbility|GetFPReplicatedWeaponActor))
          (CallFunction|ChangeSelectMode (Class|RFGameplayAbility|GetTPReplicatedWeaponActor)))
        (:OnCompleted
          ;[1 1 1] End ability when dead
          (Ability|EndAbility :!label _label))
        (:OnBlendOut
          (goto _label))
        (:OnInterrupted
          (goto _label))
        (:OnCancelled
          (goto _label))))
    (:else
      (goto _label))))

(event Ability|EventOnEndAbility
  (params (bWasCancelled :type Boolean))
  (Ability|GameplayEffect|RemoveLooseGameplayTags (Ability|GetOwningActorfromActorInfo) (GameplayTags|MakeLiteralGameplayTagContainer "(GameplayTags=((TagName=\"Ability.Weapon.Event.BlockFire\")))")))

(fn ChangeSelectMode
  (params (Object :type Object%20Object%20Reference))
  (bind _asrfweapon_base (Utilities|Casting|CastToRFWeaponBase Object))
  (if (Variables|Default|GetIs%20Up%20Select)
    (Class|RFWeaponBase|UpSelectMode _asrfweapon_base)
    (else
      (Class|RFWeaponBase|DownSelectMode _asrfweapon_base))))