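; Gameplay ability for the SCAR-L's fire-select-down action.
; It overrides only the activation check, which fetches the first-person replicated weapon actor from the actor info and casts it to B_WeaponBase.
; Activation is allowed only while that weapon's FireSelectMode is not Safety.
; The activate and end events are disabled stubs, so any actual mode switching comes from outside this Blueprint's graphs.
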(event Ability|EventActivateAbility
  (|CallParentFunction) ; This node is disabled and will not be called.\nDrag off pins to build functionality.
)

(event Ability|EventOnEndAbility
  (params (bWasCancelled :type Boolean))
  (|CallParentFunction bWasCancelled) ; This node is disabled and will not be called.\nDrag off pins to build functionality.
)

(fn K2CanActivateAbility
  (params (ActorInfo :type Gameplay%20Ability%20Actor%20Info%20Structure) (Handle :type Gameplay%20Ability%20Spec%20Handle%20Structure))
  (bind _returnvalue (Class|RFGameplayAbility|GetFPReplicatedWeaponActorbyActorInfo ActorInfo))
  (Utilities|IsValid _returnvalue
    (:Is%20Valid
      (bind _asb_weapon_base (Utilities|Casting|CastToB_WeaponBase _returnvalue)
        (:then
          (return "" (Utilities|Enum|NotEqual(Enum) (Variables|/Script/RT_FPS.RFWeaponBase|GetFireSelectMode _asb_weapon_base) "Safety")))
        (:CastFailed
          (return "" false))))))