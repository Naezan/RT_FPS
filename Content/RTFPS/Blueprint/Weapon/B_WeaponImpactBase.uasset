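; Base weapon impact actor that plays a surface-specific bullet impact effect, then cleans itself up.
; FireEffect looks up the surface type's name in DT_BulletImpactData and spawns that row's effect at the hit location, oriented along the impact normal.
; It then polls the spawned effect on a repeating retriggerable delay and destroys the actor once the effect is no longer valid.
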(event EventBeginPlay)

(event Collision|EventActorBeginOverlap
  (params (OtherActor :type Actor%20Object%20Reference)))

(event EventTick
  (params (DeltaSeconds :type Float%20%28single-precision%29)))

(event EventFireEffect
  (params (IsFP :type Boolean) (Location :type Vector :default "0, 0, 0") (ImpactNormal :type Vector :default "0, 0, 0") (SurfaceType :type EPhysicalSurface%20Enum :default "SurfaceType_Default"))
  (Utilities|FlowControl|Sequence
    (:then_0
      (bind _returnvalue (Utilities|GetDataTableRow "/Game/RTFPS/PhysicsData/DT_BulletImpactData.DT_BulletImpactData" (Utilities|String|StringToName (Utilities|String|EnumtoString SurfaceType)))
        (:then
          (bind _returnvalue_2 (Niagara|SpawnSystematLocation (Utilities|Struct|BreakS_BulletImpactInfo _returnvalue) Location (Math|Conversions|RotationFromXVector ImpactNormal)))
          (Variables|Niagara-Impact|SetLastAttachedImpactEffect _returnvalue_2))))
    (:then_1
      ;[1 1 1] ResetEffectPool
      (Utilities|FlowControl|RetriggerableDelay 2.0 :!label _label)
      (if (Utilities|IsValid (Variables|Niagara-Impact|GetLastAttachedImpactEffect))
        (goto _label)
        (else
          (Actor|DestroyActor))))))

(fn ConstructionScript)